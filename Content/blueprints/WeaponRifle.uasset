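; Rifle weapon Blueprint that prototypes firing and ammo consumption through debug messages.
; On BeginPlay it enables input from the first player controller and calls AttachWeapon, which is not defined in this graph.
; Pressing Space Bar decrements AmmoAttribute and prints the remaining count, or prints an empty notice when none is left.
; No projectile, trace or damage logic is present.
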(event Collision|EventActorBeginOverlap
  (params (OtherActor :type Actor%20Object%20Reference)))

(event EventBeginPlay
  (Input|EnableInput (Game|GetPlayerController 0))
  (Class|WeaponBase|AttachWeapon))

(event Input|KeyboardEvents|SpaceBar
  (params (Key :type Key%20Structure))
  (:Pressed
    (if (> (Variables|Default|GetammoAttribute) 0)
      (Development|PrintString "Weapon fired")
      (bind _output_get (Variables|Default|SetammoAttribute (- (Variables|Default|GetammoAttribute) 1)))
      (Development|PrintString (Utilities|String|ToString(Integer) _output_get))
      (else
        (Development|PrintString "Empty")))))

(fn ConstructionScript)